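; Stealth-game enemy AI character that patrols, investigates noises, chases the spotted player and melee-attacks to send them to a checkpoint.
; Tick chooses chasing, target-point patrol or random roaming through boolean flags, using AIMoveTo and per-state walk speeds.
; PawnSensing drives delayed sight detection with retriggerable loss of interest, plus noise investigation.
; An attack montage notify runs a hand-socket sphere trace; a DoOnce resets after the montage while still Hostile.
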(event `self.ReceiveBeginPlay`
  ; Comment
  (`|ExecutionSequence`
    (:`then_0`
      (bind _returnvalue (`GameplayStatics.GetActorOfClass` "/Game/StealthGame/Core/Pickups/BP_DistractionItemPawn.BP_DistractionItemPawn_C"))
      (set `self.DistractionRef` _returnvalue))))

(event `self.ReceiveTick`
  (params (DeltaSeconds :type "Float (single-precision)"))
  (bind _bplayervari (`self.bPlayerVari`))
  (if (`self.bCanMove`)
    (if _bplayervari
      (`self.Chase player`)
      (elif (`self.BtargetPointMove`)
        (`self.MoveToNextPatrolPoint`)
        (else
          (`self.Patrolrandom`))))
    (elif _bplayervari
      (`self.Chase player`))))

(event `self.PawnSensing.OnSeePawn`
  (params (Pawn :type "Pawn Object Reference"))
  (`|ExecutionSequence`
    (:`then_0`
      (cast `/Game/StealthGame/Core/Characters/PlayerCharacter/BP_ThirdPersonCharacterCustom` Pawn
        (:`then`
          (`KismetSystemLibrary.PrintString` "What's that?1")
          (if (`self.bPlayerSpotted`)
            (`KismetSystemLibrary.PrintString` "Stop Right There!" true true (struct :`R` 1.0 :`G` 4.7e-05 :`B` 0.011252 :`A` 1.0))
            (set `self.bPlayerVari` true)
            (else
              (set `self.bPlayerSpotted` true)
              (`KismetSystemLibrary.Delay` 3.0)
              (if (`self.bPlayerSpotted`)
                (set `self.bPlayerVari` true)))))
        (:`CastFailed`
          (set `self.bPlayerVari` false))))
    (:`then_1`
      (`KismetSystemLibrary.RetriggerableDelay` 1.0)
      (set `self.bPlayerSpotted` false)
      (set `self.bPlayerVari` false))))

(event `Chase player`
  (`self.update walk speed` 600.0)
  (if (`self.bPlayerVari`)
    (`|AIMoveTo` self (0.0 0.0 0.0) (`GameplayStatics.GetPlayerCharacter` 0) 100.0
      (:`OnSuccess`
        (`self.Attacking`)
        (set `self.bPlayerVari` true)))
    (else
      (set `self.bPlayerVari` false))))

(event `Patrolrandom`
  (`self.update walk speed` 300.0)
  (set `self.bCanMove` false)
  (`|AIMoveTo` self (`NavigationSystemV1.K2_GetRandomReachablePointInRadius` (`self.K2_GetActorLocation`) 2000.0 null null) null 0.0
    (:`OnSuccess`
      (`KismetSystemLibrary.Delay` 3.0)
      (set `self.bCanMove` true))))

(event `MoveToNextPatrolPoint`
  (`self.update walk speed` 250.0)
  (set `self.bCanMove` false)
  (`|AIMoveTo` self (0.0 0.0 0.0) (`|GetArrayItem` (`self.TargetPoints`) (`self.PatrolTargerPointIndex`)) 50.0
    (:`then`
      (`self.SetNextPatrolPointIndex`)
      (`KismetSystemLibrary.Delay` 5.0)
      (set `self.bCanMove` true))))

(event `SetNextPatrolPointIndex`
  (set `self.PatrolTargerPointIndex` (mod (+ (`self.PatrolTargerPointIndex`) 1) (`KismetArrayLibrary.Array_Length` (`self.TargetPoints`)))))

(event `self.PawnSensing.OnHearNoise`
  (params (Instigator :type "Pawn Object Reference") (Location :type "Vector Structure (by ref)") (Volume :type "Float (single-precision)"))
  (`self.update walk speed` 200.0)
  (set `self.bCanMove` false)
  (`KismetSystemLibrary.PrintString` "What was that?1")
  (`|AIMoveTo` self Location Instigator 1.5
    (:`OnSuccess`
      (`KismetSystemLibrary.Delay` 12.0)
      (set `self.bCanMove` true))))

(event `Attacking`
  (bind _returnvalue (`SceneComponent.GetSocketLocation` (`self.Mesh`) "hand_r"))
  ;[0.15 0.1407 0.04319 0.5] Bonk
  (`/Engine/EditorBlueprintResources/StandardMacros.DoOnce` false :!label _label ; Only Reset Attack on miss.
    (:`Completed`
      (bind _notifyname (`|PlayMontage` (`self.Mesh`) "/Game/StealthGame/Characters/Enemies/AM_Attack_01.AM_Attack_01") ; Play the AM_Attack_01
        (:`OnCompleted`
          (if (`self.bHostile`)
            (`self.ResetAttack`)))
        (:`OnNotifyBegin`
          (switch `name` _notifyname ; Pick the proper attack type(standard when there is more than one type of attack)
            (:`AttackDamage`
              (`KismetSystemLibrary.PrintString` "I'm attacking!")
              (bind (_outhits _returnvalue_2) (`KismetSystemLibrary.SphereTraceMultiForObjects` _returnvalue (+ _returnvalue (* (`self.GetActorForwardVector`) (`self.MeleeTraceDistance`))) (`self.MeleeTraceRadius`) (`|MakeArray` "ObjectTypeQuery3" :!type "EObjectTypeQuery Enum"))) ; Trace forward from hand socket.
              (if _returnvalue_2
                (for _array_element _outhits
                  (bind _asbp_third_person_character_custom (cast `/Game/StealthGame/Core/Characters/PlayerCharacter/BP_ThirdPersonCharacterCustom` (`.HitActor` (`GameplayStatics.BreakHitResult` _array_element))))
                  (`NiagaraFunctionLibrary.SpawnSystemAtLocation` "/Game/StealthGame/Effects/VFX/NS_TrueImpact.NS_TrueImpact" (`SceneComponent.GetSocketLocation` (`self.Mesh`) "hand_r") (struct) (0.02 0.02 0.02))
                  (`/Game/StealthGame/Core/Characters/PlayerCharacter/BP_ThirdPersonCharacterCustom.LoadCheckpoint` _asbp_third_person_character_custom)
                  (set `self.bHostile` false) ; ...and stop attacking...
                )))))))))

(event `ResetAttack`
  ;[0.15 0.1407 0.04319 0.5] Bonk
  (goto _label :!via `Reset`))

(fn `update walk speed`
  (params (`Max Walk Speed` :type "Float (double-precision)"))
  (set `CharacterMovementComponent.MaxWalkSpeed` `Max Walk Speed` (`self.CharacterMovement`)))

(fn `UserConstructionScript`)